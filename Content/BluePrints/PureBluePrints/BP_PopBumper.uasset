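; BP_PopBumper is a pinball pop bumper that knocks the ball away when it overlaps the actor.
; Bump replaces the ball's physics velocity with the direction from bumper to ball scaled by Power, and an attached sound and particle burst play.
; A timeline alpha then drives SetBumperBottom, which lowers the bottom piece and ramps the base's emissive material parameter and point light intensity together.
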(event EventBeginPlay)

(event Collision|EventActorBeginOverlap
  (params (OtherActor :type Actor%20Object%20Reference))
  (bind _asbp_pin_ball (Utilities|Casting|CastToBP_PinBall OtherActor))
  (CallFunction|Bump _asbp_pin_ball)
  (Audio|SpawnSoundAttached "/Game/Assets/Sounds/Cue_Bumper.Cue_Bumper" (Variables|Default|GetBumperBase) "None" "0, 0, 0" "0, 0, 0" "KeepRelativeOffset" false 1.0 1.0 0.0 0 0)
  (Effects|SpawnEmitteratLocation "/Game/Assets/Particles/P_Bumper.P_Bumper" (Transformation|GetWorldLocation (Variables|Default|GetBumperBase)))
  (bind _bumperalpha (Timeline|BumperTimeLine PlayFromStart)
    (:Update
      (CallFunction|SetBumperBottom _bumperalpha))))

(fn ConstructionScript)

(fn Bump
  (params (Ball :type BP%20Pin%20Ball%20Object%20Reference))
  (Physics|SetPhysicsLinearVelocity (Variables|/Game/BluePrints/PureBluePrints/BP_PinBall.BP_PinBall_C|GetBall Ball) (* (Math|Vector|GetUnitDirection(Vector) (Transformation|GetActorLocation) (Transformation|GetActorLocation Ball)) (Variables|Default|GetPower)) false "None"))

(fn SetBumperBottom
  (params (Time :type Float%20%28single-precision%29))
  (Transformation|SetRelativeLocation (Variables|Default|GetBumperBottom) (Math|Vector|Lerp(Vector) "0, 0, 0" "0, 0,-70.000000" Time) false false)
  (Rendering|Material|SetScalarParameterValueonMaterials (Variables|Default|GetBumperBase) "Emissive" (Math|Float|Lerp 0.0 2e+01 Time))
  (Rendering|Components|Light|SetIntensity (Variables|Default|GetPointLight) (Math|Float|Lerp 0.0 8e+03 Time)))