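; Pinball ball actor that simulates the roll down the table and keeps the ball on the playfield.
; Each tick it applies a mass-independent impulse along negative world X, scaled by Speed and delta time.
; A downward line trace supplies the surface normal for a second impulse that presses the ball onto the surface by Stickness.
; Ball velocity also drives the clamped volume and pitch of its Audio component.
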(event EventBeginPlay)

(event Collision|EventActorBeginOverlap
  (params (OtherActor :type Actor%20Object%20Reference)))

(event EventTick
  (params (DeltaSeconds :type Float%20%28single-precision%29))
  (bind _returnvalue (Transformation|GetVelocity))
  (bind _returnvalue_2 (Transformation|GetActorLocation))
  (bind _audio (Variables|Default|GetAudio))
  (bind _returnvalue_3 (Math|Vector|VectorLength _returnvalue))
  (bind _returnvalue_4 (/ _returnvalue_3 2e+03))
  (Utilities|FlowControl|Sequence
    (:then_0
      (Physics|AddImpulse (Variables|Default|GetBall) (Math|Vector|MakeVector (* (Variables|Default|GetSpeed) -1.0 DeltaSeconds) 0.0 0.0) "None" true)
      (bind _outhit (Collision|LineTraceByChannel _returnvalue_2 (- _returnvalue_2 "0, 0,500.000000") "TraceTypeQuery1" false 0 "None"))
      (Physics|AddImpulse (Variables|Default|GetBall) (* (* (* (.ImpactNormal (Collision|BreakHitResult _outhit)) -1.0) (Variables|Default|GetStickness)) DeltaSeconds) "None" true))
    (:then_1
      (Audio|Components|Audio|SetVolumeMultiplier _audio (Math|Float|Clamp(Float) _returnvalue_4 0.0 1.2) :!class /Script/Engine.AudioComponent)
      (Audio|Components|Audio|SetPitchMultiplier _audio (Math|Float|Clamp(Float) _returnvalue_4 0.9 1.1)))))

(fn ConstructionScript)