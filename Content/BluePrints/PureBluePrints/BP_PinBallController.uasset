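; Player controller for a pinball game that turns input actions into plunger, flipper and table-tilt actions.
; On BeginPlay it caches the plunger and sorts all flippers into left and right lists by type.
; Charge charges and releases the plunger, while flip inputs raise and lower each side's flippers.
; Tilt spends one of the game mode's TiltCount to shove every ball sideways with a direction-oriented camera shake.
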(event Custom|FindAllFlipers
  (bind _outactors (Actor|GetAllActorsOfClass "/Game/BluePrints/PureBluePrints/BP_Fliper.BP_Fliper_C"))
  (for _array_element _outactors
    (switch Utilities|FlowControl|Switch|SwitchonE_Direction (Variables|/Game/BluePrints/PureBluePrints/BP_Fliper.BP_Fliper_C|GetFliperType _array_element)
      (:NewEnumerator0
        (Utilities|Array|Add (Variables|Default|GetLeftFlipers) _array_element))
      (:NewEnumerator1
        (Utilities|Array|Add (Variables|Default|GetRightFlipers) _array_element)))))

(event Custom|FindPlunger
  (bind _outactors (Actor|GetAllActorsOfClass "/Game/BluePrints/PureBluePrints/BP_Piunger.BP_Piunger_C"))
  (Variables|Default|SetPlunger (Utilities|Array|Get(acopy) _outactors)))

(event EventBeginPlay
  (CallFunction|FindAllFlipers)
  (CallFunction|FindPlunger))

(event EventTick
  (params (DeltaSeconds :type Float%20%28single-precision%29)))

(event Input|ActionEvents|InputActionLeftFlip
  (params (Key :type Key%20Structure))
  (:Pressed
    (for _array_element (Variables|Default|GetLeftFlipers)
      (Default|FliperUp _array_element)))
  (:Released
    (for _array_element_2 (Variables|Default|GetLeftFlipers)
      (Default|FliperDown _array_element_2))))

(event Input|ActionEvents|InputActionRightFlip
  (params (Key :type Key%20Structure))
  (:Pressed
    (for _array_element (Variables|Default|GetRightFlipers)
      (Default|FliperUp _array_element)))
  (:Released
    (for _array_element_2 (Variables|Default|GetRightFlipers)
      (Default|FliperDown _array_element_2))))

(event Input|ActionEvents|InputActionCharge
  (params (Key :type Key%20Structure))
  (bind _plunger (Variables|Default|GetPlunger))
  (:Pressed
    (Default|Charge _plunger))
  (:Released
    (Default|Release _plunger)))

(event Input|ActionEvents|InputActionTiltLeft
  (params (Key :type Key%20Structure))
  (:Pressed
    (CallFunction|Tilt "NewEnumerator0")))

(event Input|ActionEvents|InputActionTiltRight
  (params (Key :type Key%20Structure))
  (:Pressed
    (CallFunction|Tilt "NewEnumerator1")))

(fn ConstructionScript)

(fn Tilt
  (params (Direction :type E_Direction%20Enum :default "NewEnumerator0"))
  (bind _playercameramanager (Variables|Default|GetPlayerCameraManager))
  (bind _returnvalue (Camera|GetCameraRotation _playercameramanager))
  (if (>= (Variables|/Game/BluePrints/PureBluePrints/BP_GameMode.BP_GameMode_C|GetTiltCount (.AsBP%20Game%20Mode (Utilities|Casting|CastToBP_GameMode (Game|GetGameMode)))) 1)
    (bind _outactors (Actor|GetAllActorsOfClass "/Game/BluePrints/PureBluePrints/BP_PinBall.BP_PinBall_C"))
    (if (>= (Utilities|Array|Length _outactors) 1)
      (for _array_element _outactors
        (Physics|AddImpulse (Variables|/Game/BluePrints/PureBluePrints/BP_PinBall.BP_PinBall_C|GetBall _array_element) (Utilities|Select :Index Direction :NewEnumerator0 "0,-500.000000, 0" :NewEnumerator1 "0,500.000000, 0") "None" true))
      (Game|Feedback|ClientStartCameraShake "/Game/BluePrints/PureBluePrints/BP_PinBallCameraShake.BP_PinBallCameraShake_C" 1.0 "UserDefined" (Utilities|Select :Index Direction :NewEnumerator0 _returnvalue :NewEnumerator1 (Math|Rotator|CombineRotators _returnvalue "0,180.000000, 0")))
      (Math|Integer|DecrementInt (Variables|/Game/BluePrints/PureBluePrints/BP_GameMode.BP_GameMode_C|GetTiltCount (.AsBP%20Game%20Mode (Utilities|Casting|CastToBP_GameMode (Game|GetGameMode))))))))