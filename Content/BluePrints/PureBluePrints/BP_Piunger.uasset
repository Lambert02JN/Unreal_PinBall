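; Plunger actor, apparently a launcher, that pulls back on Charge and snaps back on Release.
; Charge plays a timeline that slides the Piunger component along its local Y axis from rest.
; Release stops the timeline without rewinding it and quickly moves the component back to its relative origin.
; GetSpawnLocationWorld converts the local SpawnLocation to world space through the actor transform.
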(event Custom|Release
  (Utilities|FlowControl|Sequence
    (:then_0
      (bind _chargealpha (Timeline|ChargeTimeLine Stop)
        (:Update
          (Transformation|SetRelativeLocation (Variables|Default|GetPiunger) (Math|Vector|Lerp(Vector) "0, 0, 0" "0,150.000000, 0" _chargealpha) false false))))
    (:then_1
      (Components|MoveComponentTo (Variables|Default|GetPiunger) "0, 0, 0" "0, 0, 0" false false 0.1 false))))

(event Custom|Charge
  (bind _chargealpha (Timeline|ChargeTimeLine Play)
    (:Update
      (Transformation|SetRelativeLocation (Variables|Default|GetPiunger) (Math|Vector|Lerp(Vector) "0, 0, 0" "0,150.000000, 0" _chargealpha) false false))))

(event EventBeginPlay)

(event Collision|EventActorBeginOverlap
  (params (OtherActor :type Actor%20Object%20Reference)))

(event EventTick
  (params (DeltaSeconds :type Float%20%28single-precision%29)))

(fn ConstructionScript)

(fn GetSpawnLocationWorld
  (return (Math|Transform|TransformLocation (Transformation|GetActorTransform) (Variables|Default|GetSpawnLocation))))