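; BP_Post is a construction-time actor that builds a two-ended post structure between its left post and a configurable right location.
; The construction script turns PostLeft toward PostRightLocation and adds an SM_PostHalf mesh there facing back.
; A third mesh component copies PostLeft's transform and scales its X by the distance between the ends to form the connecting span.
; The event graph holds no logic.
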(event EventBeginPlay)

(event Collision|EventActorBeginOverlap
  (params (OtherActor :type Actor%20Object%20Reference)))

(event EventTick
  (params (DeltaSeconds :type Float%20%28single-precision%29)))

(fn ConstructionScript
  (bind _postrightlocation (Variables|Default|GetPostRightLocation))
  (bind _postleft (Variables|Default|GetPostLeft))
  (bind _postleft_2 (Variables|Default|GetPostLeft))
  (bind _returnvalue (Transformation|GetRelativeTransform _postleft_2))
  (bind _relativelocation (Variables|/Script/Engine.SceneComponent|GetRelativeLocation _postleft))
  (bind _scale (Math|Transform|BreakTransform _returnvalue))
  (Transformation|SetRelativeRotation (Variables|Default|GetPostLeft) (Math|Rotator|FindLookatRotation _relativelocation (Variables|Default|GetPostRightLocation)) false false)
  (bind _returnvalue_2 (AddComponent|AddStaticMeshComponent false (Math|Transform|MakeTransform _postrightlocation (Math|Rotator|FindLookatRotation _postrightlocation _relativelocation))))
  (bind _output_get (Variables|Default|SetPostRight _returnvalue_2))
  (Components|StaticMesh|SetStaticMesh _output_get "/Game/Assets/Mesh/SM_PostHalf.SM_PostHalf")
  (bind _returnvalue_3 (AddComponent|AddStaticMeshComponent false _returnvalue))
  (Transformation|SetRelativeScale3D _returnvalue_3 (Math|Vector|MakeVector (/ (Math|Vector|VectorLength (- (Variables|/Script/Engine.SceneComponent|GetRelativeLocation (Variables|Default|GetPostLeft)) (Variables|/Script/Engine.SceneComponent|GetRelativeLocation (Variables|Default|GetPostRight)))) 1e+02) (.y _scale) (.z _scale))))