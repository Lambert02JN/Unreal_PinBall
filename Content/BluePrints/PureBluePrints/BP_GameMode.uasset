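; BP_GameMode is the game mode for a pinball game, keeping a ball in play and tracking the tilt count.
; On BeginPlay it spawns a BP_PinBall at the spawn location of the first BP_Piunger found in the level.
; Each spawn resets TiltCount to MaxTiltCount and binds the ball's OnDestroyed event, so losing a ball immediately spawns a replacement with no limit.
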(event Custom|SpawnBall
  (Variables|Default|SetTiltCount (Variables|Default|GetMaxTiltCount))
  (bind _outactors (Actor|GetAllActorsOfClass "/Game/BluePrints/PureBluePrints/BP_Piunger.BP_Piunger_C"))
  (bind _returnvalue (Game|SpawnActorfromClass "/Game/BluePrints/PureBluePrints/BP_PinBall.BP_PinBall_C" (Math|Transform|MakeTransform (Default|GetSpawnLocationWorld (Utilities|Array|Get(acopy) _outactors)) "0, 0, 0" "1,1,1") "Undefined" 0 0))
  (Game|BindEventtoOnDestroyed _returnvalue (delegate Custom|OnBallDestroyed)))

(event Custom|OnBallDestroyed
  (params (DestroyedActor :type Actor%20Object%20Reference))
  (CallFunction|SpawnBall))

(event EventBeginPlay
  (CallFunction|SpawnBall)
  (Variables|Default|SetTiltCount (Variables|Default|GetMaxTiltCount)))

(event EventTick
  (params (DeltaSeconds :type Float%20%28single-precision%29)))

(fn ConstructionScript)